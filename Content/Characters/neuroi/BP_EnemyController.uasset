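; AI controller for S1Enemy pawns that turns the pawn's current state into movement or attack effects.
; On possess it caches the pawn, then polls its state every Tick, runs the matching action and resets it to IDLE, so each command fires once.
; MOVE paths to the pawn's target location, RUNAWAY to a random reachable nearby point.
; ATTACK only spawns an explosion emitter and sound, applying no damage here.
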(event `self.ReceiveBeginPlay`)

(event `self.ReceiveTick`
  (params (DeltaSeconds :type "Float (single-precision)"))
  (bind _ass1enemy (cast `S1Enemy` (`self.PossessedPawn`)))
  (bind _returnvalue (`S1Enemy.GetState` _ass1enemy))
  (switch `AiState` _returnvalue
    (:`MOVE`
      (bind _returnvalue_2 (`S1Enemy.GetTargetLocation` _ass1enemy))
      (`self.Enemy_move` _returnvalue_2)
      (`S1Enemy.SetMoveState` _ass1enemy "IDLE"))
    (:`ATTACK`
      (`self.Enemy_attack`)
      (`S1Enemy.SetMoveState` _ass1enemy "IDLE"))
    (:`RUNAWAY`
      (`self.Enemy_runaway`)
      (`S1Enemy.SetMoveState` _ass1enemy "IDLE"))))

(event `self.ReceivePossess`
  (params (PossessedPawn :type "Pawn Object Reference"))
  (bind _ass1enemy (cast `S1Enemy` PossessedPawn))
  (set `self.PossessedPawn` _ass1enemy))

(fn `Enemy_attack`
  (bind _returnvalue (`self.K2_GetActorLocation`))
  (`GameplayStatics.SpawnEmitterAtLocation` "/Game/StarterContent/Particles/P_Explosion.P_Explosion" _returnvalue (struct) (4.0 4.0 4.0))
  (`GameplayStatics.SpawnSoundAtLocation` "/Game/StarterContent/Audio/Explosion01.Explosion01" _returnvalue (struct) 0.1 1.0 0.0 null null))

(fn `Enemy_move`
  (params (TargetLocation :type "Vector Structure"))
  (`self.MoveToLocation` TargetLocation -1.0 true true false true null))

(fn `Enemy_runaway`
  (`self.MoveToLocation` (`NavigationSystemV1.K2_GetRandomReachablePointInRadius` (`self.K2_GetActorLocation`) 1000.0 null null) -1.0 true true false true null))

(fn `UserConstructionScript`)