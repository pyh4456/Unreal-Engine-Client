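; BP_AimHUD is a HUD that shows a crosshair while the player character is aiming.
; Each DrawHUD call casts the player character to BP_character and checks its Aiming flag.
; When the flag is set, it draws the Crosshair1 texture at a fixed pixel size, centered on the screen.
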(event `self.ReceiveDrawHUD`
  (params (SizeX :type Integer) (SizeY :type Integer))
  (bind _asbp_character (cast `/Game/Characters/501/BP_character` (`GameplayStatics.GetPlayerCharacter` 0)))
  (if (`/Game/Characters/501/Sanya_V_Litvyak/BP_sanya.aiming` _asbp_character)
    (`self.DrawTexture` "/Game/weapon/Texture2D/crosshair1.crosshair1" (`KismetMathLibrary.Conv_IntToDouble` (- (/ SizeX 2) 32)) (`KismetMathLibrary.Conv_IntToDouble` (- (/ SizeY 2) 32)) 64.0 64.0 0.0 0.0 1.0 1.0)))

(fn `UserConstructionScript`)